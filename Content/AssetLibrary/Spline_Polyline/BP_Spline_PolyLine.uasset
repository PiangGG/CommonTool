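; Construction-script Blueprint that draws a styled polyline or band along an editable spline, optionally closed into a loop.
; CreatSpline adds one spline mesh per segment, with MeshDirection selecting the plane mesh, forward axis and up vector, and Width setting scale.
; A valid StyleLibrary material becomes a dynamic instance driven by color, brightness and stroke settings.
; Segments are attached and positioned only in that branch, with optional overridden tangents.
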(fn `CreatSpline`
  (bind _returnvalue (`KismetMathLibrary.MakeVector` 0.0 0.0 1.0))
  (bind _meshdirection (`self.MeshDirection`))
  (bind _meshdirection_2 (`self.MeshDirection`))
  (bind _spline (`self.Spline`))
  (bind _splinetangent_0 (`self.SplineTangent=0`))
  (bind _returnvalue_2 (/ (`self.Width`) 50.0))
  (bind _value (`BlueprintMapLibrary.Map_Find` (`self.Style_library`) (`|GetEnumeratorNameAsString` (`self.Style`))))
  (for _index (range (+ (- (`SplineComponent.GetNumberOfSplinePoints` (`self.Spline`)) (select `bool` (`self.Loop`) :`false` 2 :`true` 1)) 1))
    (`SplineComponent.SetSplinePointType` (`self.Spline`) _index (`self.Spline_Type`) true) ; 设置样条线的类型
    (bind _returnvalue_3 (`AddComponent|NODE_AddSplineMeshComponent-8`))
    (`StaticMeshComponent.SetStaticMesh` _returnvalue_3 (select `byte` _meshdirection :`0` "/CommonTool/AssetLibrary/Spline_Polyline/Mesh/plane_Center.plane_Center" :`1` "/CommonTool/AssetLibrary/Spline_Polyline/Mesh/Plane_Side.Plane_Side" :`2` "/CommonTool/AssetLibrary/Spline_Polyline/Mesh/plane_Center.plane_Center" :!type "StaticMesh Object Reference"))
    (`SplineMeshComponent.SetForwardAxis` _returnvalue_3 (select `byte` _meshdirection :`0` "X" :`1` "X" :`2` "Y" :!type "ESplineMeshAxis Enum") true)
    (`SplineMeshComponent.SetSplineUpDir` _returnvalue_3 (select `byte` _meshdirection :`0` _returnvalue :`1` _returnvalue :`2` (`KismetMathLibrary.MakeVector` 0.0 0.0 -1.0)) true)
    (`SplineMeshComponent.SetStartScale` _returnvalue_3 (`KismetMathLibrary.MakeVector2D` _returnvalue_2 _returnvalue_2) true)
    (`SplineMeshComponent.SetEndScale` _returnvalue_3 (`KismetMathLibrary.MakeVector2D` _returnvalue_2 _returnvalue_2) true)
    (`PrimitiveComponent.SetMassScale` _returnvalue_3 "None" 1.0)
    (`/Engine/EditorBlueprintResources/StandardMacros.IsValid` _value
      (:`Is Valid`
        (bind _returnvalue_4 (`PrimitiveComponent.CreateDynamicMaterialInstance` _returnvalue_3 0 _value "None"))
        (`MaterialInstanceDynamic.SetScalarParameterValue` _returnvalue_4 "E_Brightness" (`self.Brightness`))
        (`MaterialInstanceDynamic.SetVectorParameterValue` _returnvalue_4 "E_Color" (`self.Color`))
        (`MaterialInstanceDynamic.SetScalarParameterValue` _returnvalue_4 (select `byte` _meshdirection_2 :`0` "None" :`1` "None" :`2` "None" :!type "Name") (select `byte` (`self.MeshDirection`) :`0` 0.0 :`1` 0.0 :`2` 0.0))
        (`MaterialInstanceDynamic.SetScalarParameterValue` _returnvalue_4 "UV_Rotation" (select `byte` _meshdirection_2 :`0` 0.0 :`1` 0.0 :`2` 0.0))
        (bind (_location _tangent) (`SplineComponent.GetLocationAndTangentAtSplinePoint` _spline _index "Local"))
        (bind (_location_2 _tangent_2) (`SplineComponent.GetLocationAndTangentAtSplinePoint` _spline (+ _index 1) "Local"))
        (`MaterialInstanceDynamic.SetScalarParameterValue` _returnvalue_4 (select `byte` _meshdirection_2 :`0` "None" :`1` "None" :`2` "None" :!type "Name") (/ (`KismetMathLibrary.VSize` (- _location _location_2)) (select `byte` (`self.MeshDirection`) :`0` 0.0 :`1` 0.0 :`2` 0.0)))
        (`MaterialInstanceDynamic.SetScalarParameterValue` _returnvalue_4 "Stroke_Swich" (select `bool` (`self.Open_Stroke`) :`true` 1.0))
        (`MaterialInstanceDynamic.SetScalarParameterValue` _returnvalue_4 "Stroke_Width" (`KismetMathLibrary.MapRangeClamped` (`self.Stroke_Width`) 0.0 1.0 0.999 1.0002))
        (`SceneComponent.K2_AttachToComponent` _returnvalue_3 (`self.Spline`) "None" "KeepRelative" "KeepRelative" "KeepRelative" true)
        (`SplineMeshComponent.SetStartAndEnd` _returnvalue_3 _location (select `bool` _splinetangent_0 :`false` _tangent) _location_2 (select `bool` _splinetangent_0 :`false` _tangent_2 :`true` (1.0 0.0 0.0)) true)))))

(fn `UserConstructionScript`
  (`SplineComponent.SetClosedLoop` (`self.Spline`) (`self.Loop`) true)
  (`self.CreatSpline`))