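; BP_DeviceLine is an actor that draws a thin line with orange-red material color through a supplied list of locations.
; ReSetLocations destroys the old segment meshes, rebuilds the spline from the locations in local space, then calls CreatSpline.
; CreatSpline adds a spline mesh between each pair of neighboring points, setting point types to Constant and reusing the start point's tangent at both ends.
; Each segment gets its own dynamic material and is tracked in LineMeshs for cleanup.
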(event `self.ReSetLocations`
  (params (locations :type "Array of Vector Structure (by ref)"))
  (bind _splinecomponent (`self.SplineComponent`))
  (bind _linemeshs (`self.LineMeshs`))
  (for _array_element _linemeshs
    (`ActorComponent.K2_DestroyComponent` _array_element))
  (`KismetArrayLibrary.Array_Clear` _linemeshs)
  (`SplineComponent.ClearSplinePoints` _splinecomponent true)
  (for _array_element_2 locations
    (`SplineComponent.AddSplinePoint` _splinecomponent _array_element_2 "Local" true))
  (`self.CreatSpline`))

(fn `CreatSpline`
  (bind _returnvalue (/ 0.1 20.0))
  (bind _splinecomponent (`self.SplineComponent`))
  (bind _returnvalue_2 (`SplineComponent.GetNumberOfSplinePoints` (`self.SplineComponent`)))
  (if (>= _returnvalue_2 2)
    (for _index (range (+ (- _returnvalue_2 2) 1))
      (`SplineComponent.SetSplinePointType` (`self.SplineComponent`) _index "Constant" true) ; 设置样条线的类型
      (bind _returnvalue_3 (`AddComponent|NODE_AddSplineMeshComponent-0`))
      (`StaticMeshComponent.SetStaticMesh` _returnvalue_3 (select `byte` 0 :`0` null :`1` null :`2` null :!type "StaticMesh Object Reference"))
      (`SplineMeshComponent.SetForwardAxis` _returnvalue_3 (select `byte` 0 :`0` "X" :`1` "X" :`2` "X" :!type "ESplineMeshAxis Enum") true)
      (`SplineMeshComponent.SetSplineUpDir` _returnvalue_3 (select `byte` 0 :`0` (0.0 0.0 0.0) :`1` (0.0 0.0 0.0) :`2` (0.0 0.0 0.0) :!type "Vector Structure") true)
      (`SplineMeshComponent.SetStartScale` _returnvalue_3 (`KismetMathLibrary.MakeVector2D` _returnvalue _returnvalue) true)
      (`SplineMeshComponent.SetEndScale` _returnvalue_3 (`KismetMathLibrary.MakeVector2D` _returnvalue _returnvalue) true)
      (`PrimitiveComponent.SetMassScale` _returnvalue_3 "None" 1.0)
      (bind _returnvalue_4 (`PrimitiveComponent.CreateDynamicMaterialInstance` _returnvalue_3 0 null "None"))
      (`MaterialInstanceDynamic.SetScalarParameterValue` _returnvalue_4 "E_Brightness" 1.0)
      (`MaterialInstanceDynamic.SetVectorParameterValue` _returnvalue_4 "E_Color" (struct :`R` 1.0 :`G` 0.108427 :`A` 1.0))
      (`MaterialInstanceDynamic.SetScalarParameterValue` _returnvalue_4 (select `byte` 0 :`0` "None" :`1` "None" :`2` "None" :!type "Name") (select `byte` 0 :`0` 0.0 :`1` 0.0 :`2` 0.0))
      (`MaterialInstanceDynamic.SetScalarParameterValue` _returnvalue_4 "UV_Rotation" (select `byte` 0 :`0` 0.0 :`1` 0.0 :`2` 0.0))
      (bind (_location _tangent) (`SplineComponent.GetLocationAndTangentAtSplinePoint` _splinecomponent _index "Local"))
      (bind _location_2 (`SplineComponent.GetLocationAndTangentAtSplinePoint` _splinecomponent (+ _index 1) "Local"))
      (`MaterialInstanceDynamic.SetScalarParameterValue` _returnvalue_4 (select `byte` 0 :`0` "None" :`1` "None" :`2` "None" :!type "Name") (/ (`KismetMathLibrary.VSize` (- _location _location_2)) (select `byte` 0 :`0` 0.0 :`1` 0.0 :`2` 0.0)))
      (`MaterialInstanceDynamic.SetScalarParameterValue` _returnvalue_4 "Stroke_Swich" 0.0)
      (`MaterialInstanceDynamic.SetScalarParameterValue` _returnvalue_4 "Stroke_Width" (`KismetMathLibrary.MapRangeClamped` 0.0 0.0 1.0 0.999 1.0002))
      (`SceneComponent.K2_AttachToComponent` _returnvalue_3 (`self.SplineComponent`) "None" "KeepRelative" "KeepRelative" "KeepRelative" true)
      (`SplineMeshComponent.SetStartAndEnd` _returnvalue_3 _location (select `bool` false :`false` _tangent) _location_2 (select `bool` false :`false` _tangent :`true` (1.0 0.0 0.0)) true)
      (`KismetArrayLibrary.Array_AddUnique` (`self.LineMeshs`) _returnvalue_3))))

(fn `UserConstructionScript`)